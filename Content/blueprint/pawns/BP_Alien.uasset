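; BP_Alien is an enemy pawn that chases and attacks the player until killed.
; It re-issues AIMoveTo at player controller 0, and Tick pauses movement to play an attack montage when the player is in range.
; DamagePlayer applies hit damage but has no caller here.
; AnyDamage sets Health to Damage minus Health; at zero or below, KillAI updates the marine's kill counter and Mars game mode before delayed destruction.
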(event `self.ReceiveBeginPlay`
  (if (`self.Is Alive`) :!label _label
    (`|AIMoveTo` self (0.0 0.0 0.0) (`GameplayStatics.GetPlayerController` 0)
      (:`OnSuccess`
        _)
      (:`OnFail`
        _))
    (`KismetSystemLibrary.Delay` 0.2)
    (goto _label)))

(event `self.ReceiveTick`
  (params (DeltaSeconds :type "Float (single-precision)"))
  (if (`self.Can Attack`)
    (`ActorComponent.Deactivate` (`self.CharacterMovement`))
    (`|PlayMontage` (`self.Mesh`) "/Game/Characters/Enemy_Great_Spider/Animations/AM_AlienAttack.AM_AlienAttack"
      (:`OnCompleted`
        (`ActorComponent.Activate` (`self.CharacterMovement`) false)))))

(event `self.ReceiveAnyDamage`
  (params (Damage :type "Float (single-precision)") (DamageType :type "DamageType Object Reference") (InstigatedBy :type "Controller Object Reference") (DamageCauser :type "Actor Object Reference"))
  (if (`self.Is Alive`)
    (bind _output_get (set `self.Health` (- Damage (`self.Health`))))
    (if (<= _output_get 0.0)
      (`self.Kill AI`)
      (`KismetSystemLibrary.Delay` 3.0)
      (`self.K2_DestroyActor`))))

(fn `Can Attack`
  (returns (ReturnValue :type Boolean))
  (return (and (`self.Is Within Attack Range`) (not (`self.IsAttacking`)) (`self.Is Alive`))))

(fn `Damage Player`
  (if (`self.Is Alive`)
    (`GameplayStatics.ApplyDamage` (`GameplayStatics.GetPlayerCharacter` 0) (`self.Damage Per Hit`))))

(fn `Is Alive`
  (returns (ReturnValue :type Boolean))
  (return (not (`self.isDead`))))

(fn `Is Within Attack Range`
  (returns (ReturnValue :type Boolean))
  (return (< (`self.GetDistanceTo` (`GameplayStatics.GetPlayerCharacter` 0)) (`self.Attack Range`))))

(fn `IsAttacking`
  (returns (ReturnValue :type Boolean))
  (return (`AnimInstance.Montage_IsPlaying` (`SkeletalMeshComponent.GetAnimInstance` (`self.Mesh`)) "/Game/Characters/Enemy_Great_Spider/Animations/AM_AlienAttack.AM_AlienAttack")))

(fn `Kill AI`
  (bind _charactermovement (`self.CharacterMovement`))
  (set `self.isDead` true)
  (`MovementComponent.StopMovementImmediately` _charactermovement)
  (`ActorComponent.Deactivate` _charactermovement)
  (`self.SetActorEnableCollision` false)
  (bind _asbp_c_marine (cast `/Game/blueprint/pawns/BP_C_Marine` (`GameplayStatics.GetPlayerCharacter` 0)))
  (`/Game/blueprint/pawns/BP_C_Marine.Increase Kill Counter` _asbp_c_marine)
  (bind _asbp_mars_gm (cast `/Game/blueprint/GameModes/BP_Mars_GM` (`GameplayStatics.GetGameMode`)))
  (`/Game/blueprint/GameModes/BP_Mars_GM.Register Alien Death` _asbp_mars_gm self))

(fn `UserConstructionScript`)